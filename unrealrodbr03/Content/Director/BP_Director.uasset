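; BP_Director is an unfinished director Blueprint meant to track zombies and spawners.
; BeginPlay queries for actors, but the loop feeding zombies into OnZombieSpawned is disconnected, while Tick prints the Zombies array length.
; OnZombieSpawned and Onspwnd store actors and bind click or release events, and ZombieKilled duplicates the add logic instead of removing.
; Onzombie is an empty stub, with an unused calculation capping spawn count by MAxzombi.
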(event EventBeginPlay
  (Utilities|FlowControl|Sequence
    (:then_0
      (bind _outactors (Actor|GetAllActorsOfClass "/Game/zombies/blueprint/BP-zombie.BP-zombie_C")))
    (:then_1
      (bind _outactors_2 (Actor|GetAllActorsOfClass 0))
      (for _array_element _outactors_2
        _))))

(event EventTick
  (params (DeltaSeconds :type Float%20%28single-precision%29))
  (Development|PrintString (Utilities|String|Append "Zombies R" (Utilities|String|ToString(Integer) (Utilities|Array|Length (Variables|Default|GetZombies)))) true true "(R=0.000000,G=0.660000,B=1.000000,A=1.000000)" 0.0))

(fn ConstructionScript)

(fn OnZombieSpawned
  (params (Zombie :type BP-zombie%20Object%20Reference))
  (Utilities|Array|Add (Variables|Default|GetZombies) Zombie)
  (EventDispatchers|BindEventtoOnClicked Zombie (EventDispatchers|CreateEvent :!event BPDirectorAutoGenFunc)))

(fn BPDirectorAutoGenFunc
  (params (TouchedActor :type Actor%20Object%20Reference) (ButtonPressed :type Key%20Structure :default "None")))

(fn ZombieKilled
  (params (Zombie :type BP-zombie%20Object%20Reference))
  (Utilities|Array|Add (Variables|Default|GetZombies) Zombie)
  (EventDispatchers|BindEventtoOnClicked Zombie (EventDispatchers|CreateEvent :!event BPDirectorAutoGenFunc)))

(fn Onspwnd
  (params (Hspwan :type BP%20Sky%20Sphere%20Object%20Reference))
  (Utilities|Array|Add (Variables|Default|GetHspowners) Hspwan)
  (EventDispatchers|BindEventtoOnReleased Hspwan (EventDispatchers|CreateEvent :!event None)))

(fn Onzombie
  (params (count :type Integer) (location :type Vector)))